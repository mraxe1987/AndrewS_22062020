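; BP_WallLight_Automatic is a wall light that switches itself on and off by proximity.
; Box begin and end overlap events directly set the PointLight intensity to a fixed bright value or to zero, with no filtering of the overlapping actor.
; A SwitchLight function offers the same on/off toggle from a boolean, but the overlap events do not call it.
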(event `self.Box.OnComponentBeginOverlap`
  (params (OverlappedComponent :type "PrimitiveComponent Object Reference") (OtherActor :type "Actor Object Reference") (OtherComp :type "PrimitiveComponent Object Reference") (OtherBodyIndex :type Integer) (bFromSweep :type Boolean) (SweepResult :type "HitResult Structure (by ref)"))
  (`LightComponent.SetIntensity` (`self.PointLight`) 4500.0))

(event `self.Box.OnComponentEndOverlap`
  (params (OverlappedComponent :type "PrimitiveComponent Object Reference") (OtherActor :type "Actor Object Reference") (OtherComp :type "PrimitiveComponent Object Reference") (OtherBodyIndex :type Integer))
  (`LightComponent.SetIntensity` (`self.PointLight`) 0.0))

(fn `SwitchLight`
  (params (`On/Off` :type Boolean))
  (set `self.On/Off` `On/Off`)
  (if (`self.On/Off`)
    (`LightComponent.SetIntensity` (`self.PointLight`) 4500.0)
    (else
      (`LightComponent.SetIntensity` (`self.PointLight`) 0.0))))

(fn `UserConstructionScript`)