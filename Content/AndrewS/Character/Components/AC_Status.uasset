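; Character status component that tracks health and stamina, both starting at their maximums on BeginPlay.
; Damage and stamina-loss functions subtract clamped amounts, and damage that empties health fires the OnDeath dispatcher.
; Tick prints both values on screen for debugging and restores stamina by a fixed amount every frame, not scaled by delta time.
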(event `self.ReceiveBeginPlay`
  (set `self.CurrentHP` (`self.MaxHP`))
  (set `self.CurrentStamina` (`self.MaxStamina`)))

(event `self.ReceiveTick`
  (params (DeltaSeconds :type "Float (single-precision)"))
  (`KismetSystemLibrary.PrintString` (`KismetStringLibrary.Conv_DoubleToString` (`self.CurrentHP`)) true true (struct :`R` 1.0 :`B` 0.02448 :`A` 1.0) DeltaSeconds)
  (`KismetSystemLibrary.PrintString` (`KismetStringLibrary.Conv_DoubleToString` (`self.CurrentStamina`)) true true (struct :`G` 0.66 :`B` 1.0 :`A` 1.0) DeltaSeconds)
  ;[1 1 1] Восстановление выносливости
  (set `self.CurrentStamina` (`KismetMathLibrary.FClamp` (+ (`self.CurrentStamina`) (`self.RestoreStamina`)) 0.0 (`self.MaxStamina`))))

(fn `MakeDamage/Health`
  (params (Value :type "Float (double-precision)"))
  (bind _output_get (set `self.CurrentHP` (`KismetMathLibrary.FClamp` (- (`self.CurrentHP`) Value) 0.0 (`self.MaxHP`))))
  (if (<= _output_get 0.0)
    (`self.OnDeath`)))

(fn `MakeStamina/LoseStamina`
  (params (Value :type "Float (double-precision)"))
  (set `self.CurrentStamina` (`KismetMathLibrary.FClamp` (- (`self.CurrentStamina`) Value) 0.0 (`self.MaxStamina`))))