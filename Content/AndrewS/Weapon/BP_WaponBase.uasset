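; BP_WaponBase is a base weapon actor that fires automatically in an endless delayed loop starting at BeginPlay.
; Each Fire checks and subtracts one round through the AmmoAC component, then spawns a BP_AmmoBase projectile at the Arrow transform with a firing sound.
; When empty, it plays a shutter sound instead.
; Every attempt also refreshes the Ammo text with current and maximum counts.
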(event `self.ReceiveBeginPlay`
  (`KismetSystemLibrary.Delay` 0.2 :!label _label)
  (`self.Fire`)
  (goto _label))

(event `Fire`
  (bind _ammo_ac (`self.Ammo_AC`))
  (bind _ammo_ac_2 (`self.Ammo_AC`))
  (`|ExecutionSequence`
    (:`then_0`
      (if (`/Game/AndrewS/Weapon/Ammo_AC.CheckAmmo` _ammo_ac 1)
        (`/Game/AndrewS/Weapon/Ammo_AC.SubstructAmmo` _ammo_ac 1)
        (`|SpawnActorFromClass` "/Game/AndrewS/Weapon/BP_AmmoBase.BP_AmmoBase_C" (`SceneComponent.K2_GetComponentToWorld` (`self.Arrow`)) "AlwaysSpawn" "OverrideRootScale" null null)
        (`GameplayStatics.SpawnSoundAtLocation` "/Game/DownloadLearning/StarterContent/Audio/Fire01.Fire01" (`self.K2_GetActorLocation`) (struct) 1.0 1.0 0.0 null null)
        (else
          (`GameplayStatics.SpawnSoundAtLocation` "/Engine/VREditor/Sounds/UI/Camera_Shutter.Camera_Shutter" (`self.K2_GetActorLocation`) (struct) 1.0 1.0 0.0 null null))))
    (:`then_1`
      (`TextRenderComponent.K2_SetText` (`self.Ammo`) (`|FormatText` "{Current}/{Max}" (`/Game/AndrewS/Weapon/Ammo_AC.CurrentAmmo` _ammo_ac_2) (`/Game/AndrewS/Weapon/Ammo_AC.MaxAmmo` _ammo_ac_2))))))

(fn `UserConstructionScript`)